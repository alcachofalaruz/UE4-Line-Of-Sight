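; Line-of-sight actor that follows its owner, builds a view cone blocked by obstacles and toggles visibility of other actors.
; Each tick it smooths toward the owner's location and facing, then fans line traces into a procedural mesh.
; An orthographic scene capture and MPC_LOS parameters set up the post-process sight mask.
; BPI_LOSVisbility actors, gathered once after BeginPlay, are shown or hidden using range, angle and their own visibility check.
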(event `self.ReceiveBeginPlay`
  (`KismetSystemLibrary.Delay` 0.2)
  (`self.GetAllVisbilityActors`)
  (`self.SeUpPostProcessingMaterial`))

(event `self.ReceiveTick`
  (params (DeltaSeconds :type "Float (single-precision)"))
  (`self.InterpolateRotationToOwnerRotation` DeltaSeconds)
  (`self.InterpolateLocationToOwnerLocation` DeltaSeconds)
  ;[1 1 1] Note: Remember to set Procedural mesh Component to world rotation
  (`self.DrawProceduralMesh`)
  (`self.SetPostProccesingMaterialLocation`)
  (`self.Check Actors Visbility`))

(fn `Check Actors Visbility`
  (for _array_element (`self.VisibilityActors`)
    (if (and (`self.Is Actor In Range` _array_element) (`self.Is Actor Within View Angle` _array_element))
      (bind _isvisbile (message `/Game/LineOfSight/BPI_LOSVisbility.IsVisible` _array_element (`self.K2_GetActorLocation` (`self.GetOwner`))))
      (if _isvisbile
        (message `/Game/LineOfSight/BPI_LOSVisbility.Show` _array_element)
        (else
          (message `/Game/LineOfSight/BPI_LOSVisbility.Hide` _array_element)))
      (else
        (message `/Game/LineOfSight/BPI_LOSVisbility.Hide` _array_element)))))

(fn `DrawProceduralMesh`
  (bind _points_ (`self.GetSigthPoints` (`self.LinesCheckAmount`) (`self.ViewAngle`) (`self.ViewRange`) (`self.K2_GetActorLocation`) (`self.Looking Direction`)))
  (bind _vertices (`self.PointToVertices` _points_ (`self.K2_GetActorLocation`)))
  (bind _triangles_ (`self.GetTriangles` _vertices))
  (`ProceduralMeshComponent.CreateMeshSection_LinearColor` :`self` (`self.ProceduralMesh`) :`Vertices` _vertices :`Triangles` _triangles_))

(fn `GetAllVisbilityActors`
  (bind _outactors (`GameplayStatics.GetAllActorsWithInterface` "/Game/LineOfSight/BPI_LOSVisbility.BPI_LOSVisbility_C"))
  (set `self.VisibilityActors` _outactors))

(fn `GetSigthPoints`
  (params (`Lines Amount` :type Integer) (Angle :type "Float (double-precision)") (Range :type "Float (double-precision)") (Location :type "Vector Structure") (`Center Direction` :type "Vector Structure"))
  (returns (`Points ` :type "Array of Vector Structure"))
  (locals (CurrentIndex :type Integer) (StartDirection :type "Vector Structure") (Points :type "Array of Vector Structure") (AngleStep :type "Float (double-precision)"))
  ;[1 1 1] The amount of degrees we have to increase for each line trace check
  (set `local.AngleStep` (/ (`local.Angle`) (`KismetMathLibrary.Conv_IntToDouble` (- (`local.Lines Amount`) 1))))
  ;[1 1 1] The direction we are going to start the lines tracing -(angle/2)
  (set `local.StartDirection` (`KismetMathLibrary.GreaterGreater_VectorRotator` (`local.Center Direction`) (`KismetMathLibrary.MakeRotator` 0.0 0.0 (* (/ (`local.Angle`) 2.0) -1.0))))
  (for _index (range (`local.Lines Amount`))
    (set `local.CurrentIndex` _index)
    (bind _outhit (`KismetSystemLibrary.LineTraceSingle` (`local.Location`) (+ (* (`KismetMathLibrary.GreaterGreater_VectorRotator` (`local.StartDirection`) (`KismetMathLibrary.MakeRotator` 0.0 0.0 (* (`local.AngleStep`) (`KismetMathLibrary.Conv_IntToDouble` (`local.CurrentIndex`))))) (`local.Range`)) (`local.Location`)) "TraceTypeQuery3"))
    (bind (_bblockinghit _binitialoverlap _time _distance _location _impactpoint _normal _impactnormal _physmat _hitactor _hitcomponent _hitbonename _hititem _faceindex _tracestart _traceend) (`GameplayStatics.BreakHitResult` _outhit))
    ;[1 1 1] If we hit something, it means its blocking the sight, so we add the hit point, if we don't hit, we just and the end location of the check
    (`KismetArrayLibrary.Array_AddUnique` (`local.Points`) (select `bool` _bblockinghit :`false` _traceend :`true` _impactpoint)))
  (return (`local.Points`)))

(fn `GetTriangles`
  (params (Vertices :type "Array of Vector Structure (by ref)"))
  (returns (`Triangles ` :type "Array of Integer"))
  (locals (OutTriangles :type "Array of Integer"))
  ;[1 1 1] For each vertex, we'll add a triangle
  (for _index (range (+ (`KismetArrayLibrary.Array_Length` Vertices) 1))
    ;[1 1 1] Each Int Refers to a vertex
    ;;[1 1 1] Refers to the first vertex, the center
    (`KismetArrayLibrary.Array_Add` (`local.OutTriangles`))
    (bind _returnvalue (+ _index 1))
    (`KismetArrayLibrary.Array_Add` (`local.OutTriangles`) _returnvalue)
    (`KismetArrayLibrary.Array_Add` (`local.OutTriangles`) (+ _returnvalue 1)))
  (return (`local.OutTriangles`)))

(fn `InterpolateLocationToOwnerLocation`
  (params (DeltaTime :type "Float (double-precision)"))
  (`self.K2_SetActorLocation` (`KismetMathLibrary.VInterpTo` (`self.K2_GetActorLocation`) (`self.K2_GetActorLocation` (`self.GetOwner`)) DeltaTime (`self.Location Interpolation Speed`))))

(fn `InterpolateRotationToOwnerRotation`
  (params (DeltaTime :type "Float (double-precision)"))
  (set `self.Looking Direction` (`KismetMathLibrary.VInterpTo` (`self.Looking Direction`) (`self.GetActorForwardVector` (`self.GetOwner`)) DeltaTime (`self.Rotation Interpolation Speed`))))

(fn `PointToVertices`
  (params (Points :type "Array of Vector Structure") (Center :type "Vector Structure"))
  (returns (Vertices :type "Array of Vector Structure"))
  (locals (OutVertices :type "Array of Vector Structure"))
  ;[1 1 1] Adding the center as the first Vertex(Relative)
  (`KismetArrayLibrary.Array_Add` (`local.OutVertices`) (`KismetMathLibrary.MakeVector` 0.0 0.0 (`self.ZOffset`)))
  (for _array_element Points
    ;[1 1 1] Converting Absolute To Local Position
    (`KismetArrayLibrary.Array_Add` (`local.OutVertices`) (`KismetMathLibrary.MakeVector` (- (.x _array_element) (.x Center)) (- (.y _array_element) (.y Center)) (`self.ZOffset`))))
  ;[1 1 1] Adding the first point to the last index, in case we use 360 angle
  (`KismetArrayLibrary.Array_Add` (`local.OutVertices`) (`|GetArrayItem` (`local.OutVertices`) 1))
  (return (`local.OutVertices`)))

(fn `SetMeshMaterial`
  (params (Material :type "MaterialInterface Object Reference"))
  (`PrimitiveComponent.SetMaterial` (`self.ProceduralMesh`) 0 Material))

(fn `SetPostProccesingMaterialLocation`
  (`KismetMaterialLibrary.SetVectorParameterValue` "/Game/LineOfSight/Materials/MPC_LOS.MPC_LOS" "SightLineActorLocation" (`KismetMathLibrary.Conv_VectorToLinearColor` (`self.K2_GetActorLocation`))))

(fn `SeUpPostProcessingMaterial`
  (set `SceneCaptureComponent2D.OrthoWidth` (* (`self.ViewRange`) 2.15) (`self.SceneCaptureComponent2D`))
  (`SceneComponent.K2_SetRelativeTransform` (`self.SceneCaptureComponent2D`) (`KismetMathLibrary.MakeTransform` (`KismetMathLibrary.MakeVector` 0.0 0.0 (- (`self.ZOffset`) 1.0)) (struct :`Pitch` 90.0) (1.0 -1.0 -1.0)) false false)
  (`KismetMaterialLibrary.SetScalarParameterValue` "/Game/LineOfSight/Materials/MPC_LOS.MPC_LOS" "SightLineMaskHeight" (+ (.z (`self.K2_GetActorLocation`)) (`self.ZOffset`) -500.0))
  (`KismetMaterialLibrary.SetScalarParameterValue` "/Game/LineOfSight/Materials/MPC_LOS.MPC_LOS" "SightLineTexScale" (* (`self.ViewRange`) 2.0))
  (`KismetMaterialLibrary.SetVectorParameterValue` "/Game/LineOfSight/Materials/MPC_LOS.MPC_LOS" "SightLineActorLocation" (`KismetMathLibrary.Conv_VectorToLinearColor` (`self.K2_GetActorLocation`))))

(fn `UserConstructionScript`)