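; Line of sight actor component that gives its owner a vision area mesh by spawning a BP_LineOfSigth actor.
; BeginPlay sets that actor's mesh material and adds a blendable post-process material to the owner's camera.
; Tick pushes view range, angle and interpolation speeds to the actor.
; Helper functions, not called in its event graph, trace an arc of rays and build triangle-fan vertices and indices from the hits.
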(event `self.ReceiveBeginPlay`
  ;[1 1 1] Line of sight Set Up
  (bind _returnvalue (`|SpawnActorFromClass` "/Game/LineOfSight/BP_LineOfSigth.BP_LineOfSigth_C" (`Actor.GetTransform` (`self.GetOwner`)) "Undefined" "OverrideRootScale" (`self.GetOwner`) (`self.ViewAngle`) (`self.ViewRange`) (`self.ZOffset`) (`self.LinesAmount`) 0.0 0.0 null))
  (bind _output_get (set `self.LOS Actor` _returnvalue))
  (`/Game/LineOfSight/BP_LineOfSigth.SetMeshMaterial` _output_get "/Game/LineOfSight/Materials/M_LOSMesh.M_LOSMesh")
  (bind _returnvalue_2 (`KismetMaterialLibrary.CreateDynamicMaterialInstance` "/Game/LineOfSight/Materials/MI_LOSBlendable.MI_LOSBlendable"))
  (setmembers `PostProcessSettings` :`StructRef` (`CameraComponent.PostProcessSettings` (`Actor.GetComponentByClass` (`self.GetOwner`) "/Script/Engine.CameraComponent")) :`WeightedBlendables` (make `WeightedBlendables` (`|MakeArray` (make `WeightedBlendable` 1.0 _returnvalue_2)))))

(event `self.ReceiveTick`
  (params (DeltaSeconds :type "Float (single-precision)"))
  ;[1 1 1] This is needed only if we want to update the values Every frame
  (set `/Game/LineOfSight/BP_LineOfSigth.ViewRange` (`self.ViewRange`) (`self.LOS Actor`))
  (set `/Game/LineOfSight/BP_LineOfSigth.ViewAngle` (`self.ViewAngle`) (`self.LOS Actor`))
  (set `/Game/LineOfSight/BP_LineOfSigth.Location Interpolation Speed` (`self.LocationInterpSpeed`) (`self.LOS Actor`))
  (set `/Game/LineOfSight/BP_LineOfSigth.Rotation Interpolation Speed` (`self.RotationInterpSpeed`) (`self.LOS Actor`)))

(fn `ConvertToVertices`
  (params (Points :type "Array of Vector Structure") (Center :type "Vector Structure"))
  (returns (Vertices :type "Array of Vector Structure"))
  (locals (OutVertices :type "Array of Vector Structure"))
  (`KismetArrayLibrary.Array_Add` (`local.OutVertices`) (`KismetMathLibrary.MakeVector` 0.0 0.0 (`self.ZOffset`)))
  (for _array_element Points
    (`KismetArrayLibrary.Array_Add` (`local.OutVertices`) (`KismetMathLibrary.MakeVector` (- (.x _array_element) (.x Center)) (- (.y _array_element) (.y Center)) (`self.ZOffset`))))
  (`KismetArrayLibrary.Array_Add` (`local.OutVertices`) (`|GetArrayItem` (`local.OutVertices`) 1))
  (return (`local.OutVertices`)))

(fn `GetSigthPoints`
  (params (`Lines Amount` :type Integer) (Angle :type "Float (double-precision)") (Range :type "Float (double-precision)") (Location :type "Vector Structure") (`Center Direction` :type "Vector Structure"))
  (returns (`Points ` :type "Array of Vector Structure"))
  (locals (AngleStep :type "Float (double-precision)") (CurrentIndex :type Integer) (StartDirection :type "Vector Structure") (Points :type "Array of Vector Structure"))
  (set `local.AngleStep` (/ (`local.Angle`) (`KismetMathLibrary.Conv_IntToDouble` (- (`local.Lines Amount`) 1))))
  (set `local.StartDirection` (`KismetMathLibrary.GreaterGreater_VectorRotator` (`local.Center Direction`) (`KismetMathLibrary.MakeRotator` 0.0 0.0 (* (/ (`local.Angle`) 2.0) -1.0))))
  (for _index (range (`local.Lines Amount`))
    (set `local.CurrentIndex` _index)
    (bind _outhit (`KismetSystemLibrary.LineTraceSingle` (`local.Location`) (+ (`local.Location`) (* (`KismetMathLibrary.GreaterGreater_VectorRotator` (`local.StartDirection`) (`KismetMathLibrary.MakeRotator` 0.0 0.0 (* (`local.AngleStep`) (`KismetMathLibrary.Conv_IntToDouble` (`local.CurrentIndex`))))) (`self.ViewRange`))) "TraceTypeQuery3"))
    (bind (_bblockinghit _binitialoverlap _time _distance _location _impactpoint _normal _impactnormal _physmat _hitactor _hitcomponent _hitbonename _hititem _faceindex _tracestart _traceend) (`GameplayStatics.BreakHitResult` _outhit))
    (`KismetArrayLibrary.Array_AddUnique` (`local.Points`) (select `bool` _bblockinghit :`false` _traceend :`true` _impactpoint)))
  (`KismetArrayLibrary.Array_Add` (`local.Points`) (`local.Location`))
  (return (`local.Points`)))

(fn `GetTriangles`
  (params (Vertices :type "Array of Vector Structure"))
  (returns (`Triangles ` :type "Array of Integer"))
  (locals (Triangles :type "Array of Integer"))
  (for _index (range (+ (`KismetArrayLibrary.Array_Length` Vertices) 1))
    (`KismetArrayLibrary.Array_Add` (`local.Triangles`))
    (bind _returnvalue (+ _index 1))
    (`KismetArrayLibrary.Array_Add` (`local.Triangles`) _returnvalue)
    (`KismetArrayLibrary.Array_Add` (`local.Triangles`) (+ _returnvalue 1)))
  (return (`local.Triangles`)))